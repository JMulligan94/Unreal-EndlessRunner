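; Player pawn for a lane-based runner that moves constantly forward along X and switches lanes on MoveLeft and MoveRight input.
; BeginPlay reads the start lane from RunnerGameInstance and creates the HUD.
; Input starts a lane change only when none is running and LaneIndex passes the bounds check.
; Tick calls ProcessMovement, which lerps Y by one LaneWidth using a countdown from LaneChangeSpeed, which acts as a duration.
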(event `self.ReceiveBeginPlay`
  (bind _asrunner_game_instance (cast `/Game/Blueprints/RunnerGameInstance` (`GameplayStatics.GetGameInstance`)))
  (set `self.LaneIndex` (`/Game/Blueprints/RunnerGameInstance.StartLaneIndex` _asrunner_game_instance))
  (bind _returnvalue (`|CreateWidget` "/Game/UI/HUD.HUD_C"))
  (bind _output_get (set `self.HUD` _returnvalue))
  (`UserWidget.AddToViewport` _output_get 0))

(event `self.ReceiveTick`
  (params (DeltaSeconds :type "Float (single-precision)"))
  (`self.ProcessMovement`))

(event `InputAction|MoveLeft`
  (params (Key :type "Key Structure"))
  (:`Pressed`
    (bind _ismoving (`self.IsMoving`))
    (bind _canmoveleft (`self.CanMoveLeft`))
    (if (and (not _ismoving) _canmoveleft)
      (set `self.IsMovingLeft` true)
      (set `self.LaneIndex` (- (`self.LaneIndex`) 1))
      (set `self.RemainingMoveTime` (`self.LaneChangeSpeed`) :!label _label)
      (set `self.InitialPosition` (.y (`self.K2_GetActorLocation`))))))

(event `InputAction|MoveRight`
  (params (Key :type "Key Structure"))
  (:`Pressed`
    (bind _ismoving (`self.IsMoving`))
    (bind _canmoveright (`self.CanMoveRight`))
    (if (and (not _ismoving) _canmoveright)
      (set `self.IsMovingRight` true)
      (set `self.LaneIndex` (+ (`self.LaneIndex`) 1))
      (goto _label))))

(fn `CanMoveLeft`
  (returns (CanMoveLeft :type Boolean))
  (return (> (`self.LaneIndex`) 0)))

(fn `CanMoveRight`
  (returns (CanMoveRight :type Boolean))
  (bind _asrunner_game_instance (cast `/Game/Blueprints/RunnerGameInstance` (`GameplayStatics.GetGameInstance`)))
  (return (< (`self.LaneIndex`) (`/Game/Blueprints/RunnerGameInstance.LaneCount` _asrunner_game_instance))))

(fn `IsMoving`
  (returns (IsMoving :type Boolean))
  (return (or (`self.IsMovingLeft`) (`self.IsMovingRight`))))

(fn `ProcessMovement`
  (locals (DestinationPosition :type "Float (double-precision)"))
  (bind _initialposition (`self.InitialPosition`))
  ;[1 1 1] Move forwards
  (`self.K2_SetActorLocation` (+ (`self.K2_GetActorLocation`) (`KismetMathLibrary.MakeVector` (* (`self.ForwardSpeed`) (`GameplayStatics.GetWorldDeltaSeconds`)))))
  (bind _ismoving (`self.IsMoving`))
  (if _ismoving
    ;[1 1 1] Lerp changing lanes
    (set `self.RemainingMoveTime` (- (`self.RemainingMoveTime`) (`GameplayStatics.GetWorldDeltaSeconds`)))
    (bind _asrunner_game_instance (cast `/Game/Blueprints/RunnerGameInstance` (`GameplayStatics.GetGameInstance`)))
    (if (`self.IsMovingLeft`)
      (bind _lanewidth (`/Game/Blueprints/RunnerGameInstance.LaneWidth` _asrunner_game_instance))
      (set `local.DestinationPosition` (- _initialposition _lanewidth))
      (else
        (set `local.DestinationPosition` (+ _initialposition _lanewidth))))
    (`self.K2_SetActorLocation` (`KismetMathLibrary.MakeVector` (.x (`self.K2_GetActorLocation`)) (`KismetMathLibrary.Lerp` (`local.DestinationPosition`) (`self.InitialPosition`) (`KismetMathLibrary.FMax` (/ (`self.RemainingMoveTime`) (`self.LaneChangeSpeed`)))) (.z (`self.K2_GetActorLocation`))))
    (if (<= (`self.RemainingMoveTime`) 0.0)
      (set `self.IsMovingLeft` false)
      (set `self.IsMovingRight` false))))

(fn `UserConstructionScript`)