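; Platform spawner for a lane-based runner that lays PlatformActors end to end along X.
; Each platform can get a row of coins and of obstacles in a random lane, using RunnerGameInstance spawn settings.
; A wrapping index replaces entries in the platform array without destroying the old actors.
; BeginPlay spawns the initial set; the game instance's restart event resets position and index, then respawns that set inside its array-removal loop.
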(event `self.ReceiveBeginPlay`
  (bind _asrunner_game_instance (cast `/Game/Blueprints/RunnerGameInstance` (`GameplayStatics.GetGameInstance`)))
  (add `/Game/Blueprints/RunnerGameInstance.OnRestart` _asrunner_game_instance (delegate `Event OnRestart`))
  (`self.SpawnInitialPlatforms`))

(event `self.ReceiveActorBeginOverlap`
  (params (OtherActor :type "Actor Object Reference")))

(event `Event OnRestart`
  (`self.OnRestart`))

(fn `InsertPlatform`
  (params (Index :type Integer) (PlatformToAdd :type "Actor Object Reference"))
  (`KismetArrayLibrary.Array_Insert` (`self.Platforms`) PlatformToAdd Index))

(fn `OnDeath`)

(fn `OnRestart`
  (set `self.CurrentX` 0.0)
  (set `self.PlatformIndex` 0)
  (for _index (range (`KismetArrayLibrary.Array_Length` (`self.Platforms`)))
    (`self.RemovePlatform` _index)
    (`self.SpawnInitialPlatforms`)))

(fn `RemovePlatform`
  (params (Index :type Integer))
  (locals (PlatformToRemove :type "Actor Object Reference"))
  (bind _platforms (`self.Platforms`))
  (if (> (`KismetArrayLibrary.Array_Length` _platforms) Index)
    (`KismetArrayLibrary.Array_Remove` _platforms Index)))

(fn `SpawnChildrenOfType`
  (params (SpawnClass :type "/Game/Blueprints/PlatformChildActor Class Reference") (SpawnedPlatform :type "/Game/Blueprints/PlatformActor Object Reference"))
  (locals (StartX :type "Float (double-precision)"))
  (bind _currentx (`self.CurrentX`))
  (bind _asrunner_game_instance (cast `/Game/Blueprints/RunnerGameInstance` (`GameplayStatics.GetGameInstance`)))
  (bind _maxspawn (`/Game/Blueprints/RunnerGameInstance.GetMaxSpawn` _asrunner_game_instance SpawnClass))
  (bind _spawnchance (`/Game/Blueprints/RunnerGameInstance.GetSpawnChance` _asrunner_game_instance SpawnClass))
  (if (>= (- (`KismetMathLibrary.RandomIntegerInRange` 0 100) _spawnchance) 0)
    (bind _laney (`/Game/Blueprints/RunnerGameInstance.GetLaneY` _asrunner_game_instance (`KismetMathLibrary.RandomIntegerInRange` 0 (- (`/Game/Blueprints/RunnerGameInstance.LaneCount` _asrunner_game_instance) 1))))
    (set `local.StartX` (`KismetMathLibrary.RandomFloatInRange` (- _currentx (`self.PlatformLength`)) _currentx))
    (for _index (range (+ (`KismetMathLibrary.RandomIntegerInRange` 1 _maxspawn) 1))
      (bind _returnvalue (`|SpawnActorFromClass` SpawnClass (`KismetMathLibrary.Conv_VectorToTransform` (`KismetMathLibrary.MakeVector` (+ (* _index (`self.ChildMargin`)) (`local.StartX`)) _laney)) "Undefined" "OverrideRootScale" null null))
      (`/Game/Blueprints/ObstacleActor.SetOwningPlatform` _returnvalue SpawnedPlatform))))

(fn `SpawnInitialPlatforms`
  (for _ (range (`self.PlatformAmount`))
    (`self.SpawnNextPlatform`)))

(fn `SpawnNextPlatform`
  (bind _currentx (`self.CurrentX`))
  ;[1 1 1] Spawn Platform
  (bind _spawnedplatform (`self.SpawnPlatform` (`KismetMathLibrary.MakeVector` _currentx)))
  (set `self.CurrentX` (+ _currentx (`self.PlatformLength`)))
  (bind _asplatform_actor (cast `/Game/Blueprints/PlatformActor` _spawnedplatform))
  (`self.SpawnChildrenOfType` "/Game/Blueprints/CoinActor.CoinActor_C" _asplatform_actor)
  (`self.SpawnChildrenOfType` "/Game/Blueprints/ObstacleActor.ObstacleActor_C" _asplatform_actor)
  (return))

(fn `SpawnPlatform`
  (params (PlatformPosition :type "Vector Structure"))
  (returns (SpawnedPlatform :type "Actor Object Reference"))
  (bind _platformindex (`self.PlatformIndex`))
  ;[1 1 1] Spawn Platform & Update Arrays
  (bind _returnvalue (`|SpawnActorFromClass` "/Game/Blueprints/PlatformActor.PlatformActor_C" (`KismetMathLibrary.Conv_VectorToTransform` PlatformPosition) "Undefined" "OverrideRootScale" null null))
  (`self.RemovePlatform` _platformindex)
  (`self.InsertPlatform` _platformindex _returnvalue)
  (bind _result (`/Engine/EditorBlueprintResources/StandardMacros.IncrementInt` _platformindex)
    (:`  `
      (bind _output_get (set `self.PlatformIndex` _result))
      (if (== _output_get (`self.PlatformAmount`))
        (set `self.PlatformIndex` 0))
      (return _returnvalue))))

(fn `UserConstructionScript`)