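; Collectible coin actor for a runner game that is tied to the platform it belongs to.
; When its box collision overlaps the PlayerPawn, it reports the pickup to RunnerGameInstance through CollectCoin and destroys itself.
; SetOwningPlatform stores the platform and binds to its destroy event, so an uncollected coin removes itself when that platform is destroyed.
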(event `self.ReceiveBeginPlay`)

(event `self.BoxCollision.OnComponentBeginOverlap`
  (params (OverlappedComponent :type "PrimitiveComponent Object Reference") (OtherActor :type "Actor Object Reference") (OtherComp :type "PrimitiveComponent Object Reference") (OtherBodyIndex :type Integer) (bFromSweep :type Boolean) (SweepResult :type "HitResult Structure (by ref)"))
  (if (== (`GameplayStatics.GetObjectClass` OtherActor) "/Game/Blueprints/PlayerPawn.PlayerPawn_C")
    (bind _asrunner_game_instance (cast `/Game/Blueprints/RunnerGameInstance` (`GameplayStatics.GetGameInstance`)))
    (`/Game/Blueprints/RunnerGameInstance.CollectCoin` _asrunner_game_instance)
    (`self.K2_DestroyActor`)))

(event `On Owning Platform Set`
  (params (`Owning Platform` :type "/Game/Blueprints/PlatformActor Object Reference"))
  (add `/Game/Blueprints/PlatformActor.OnDestroyPlatform` `Owning Platform` (delegate `On Owning Platform Destroyed`)))

(event `On Owning Platform Destroyed`
  (params (DestroyedPlatform :type "/Game/Blueprints/PlatformActor Object Reference"))
  ;[1 1 1] Is Destroyed platform this coin's owner?
  (if (== DestroyedPlatform (`self.OwningPlatform`))
    (`self.K2_DestroyActor`)))

(fn `SetOwningPlatform`
  (params (OwningPlatform :type "/Game/Blueprints/PlatformActor Object Reference"))
  (set `self.OwningPlatform` OwningPlatform)
  (`self.On Owning Platform Set` OwningPlatform))

(fn `UserConstructionScript`)