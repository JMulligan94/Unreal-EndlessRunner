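; Game instance for a lane-based runner that holds the coin count and lane layout.
; GetLaneY converts a lane index into a Y position centred on zero from LaneWidth and LaneCount, permanently bumping an even LaneCount to the next odd number.
; CollectCoin increments NumCoins, and Restart zeroes it then fires the OnRestart dispatcher.
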(fn `CollectCoin`
  (bind _result (`/Engine/EditorBlueprintResources/StandardMacros.IncrementInt` (`self.NumCoins`))
    (:`  `
      (set `self.NumCoins` _result))))

(fn `GetLaneY`
  (params (LaneIndex :type Integer))
  (returns (LaneY :type "Float (double-precision)"))
  (bind _lanewidth (`self.LaneWidth`))
  (bind _lanecount (`self.LaneCount`))
  (if (== (mod _lanecount 2) 0)
    (bind _result (`/Engine/EditorBlueprintResources/StandardMacros.IncrementInt` _lanecount)
      (:`  `
        (bind _output_get (set `self.LaneCount` _result)))))
  (return (- (* LaneIndex _lanewidth) (* (/ _output_get 2) _lanewidth))))

(fn `Restart`
  (set `self.NumCoins` 0)
  (`self.OnRestart`))